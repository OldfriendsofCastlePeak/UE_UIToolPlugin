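; Test actor that exercises a reflection helper for calling functions by name on a referenced object and inspecting their parameters.
; A custom event invokes a three-parameter API function on that object with string arguments, while BeginPlay is empty.
; Disconnected experiments cover zero-, one- and two-argument calls and printing parameter names and types.
; A Test function prints its input and returns three fixed booleans.
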(event `self.ReceiveBeginPlay`)

(event `CustomEvent`
  (`CommonUIToolLib.CallObjectFunctionThreeParam` (`self.NewVar`) "API_ThreeParam" "one" "two" "Three"))

(fn `Test`
  (params (NewParam :type String))
  (returns (NewParam1 :type Boolean) (NewParam2 :type Boolean) (NewParam3 :type Boolean))
  (`KismetSystemLibrary.PrintString` (`KismetStringLibrary.Concat_StrStr` "传入：" NewParam))
  (return false true false))

(fn `UserConstructionScript`)