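; Value_Actor_BP is a test actor that exposes custom events and a function for exercising calls with different parameter counts.
; The no-parameter events print "Hello", while the one, two and three parameter events print each argument after a Chinese ordinal label.
; A separate function prints its single input with an "In5" label.
; BeginPlay, overlap and construction script contain no logic.
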(event `self.ReceiveBeginPlay`)

(event `API_Test`
  (`KismetSystemLibrary.PrintString` "Hello"))

(event `APITestFunc`
  (`KismetSystemLibrary.PrintString` "Hello"))

(event `API_OneParam`
  (params (NewParam :type String))
  (`KismetSystemLibrary.PrintString` (`KismetStringLibrary.Concat_StrStr` "第一个参数：" NewParam)))

(event `API_TwoParam`
  (params (NewParam :type String) (NewParam2 :type String))
  (`KismetSystemLibrary.PrintString` (`KismetStringLibrary.Concat_StrStr` "第一个参数：" NewParam "   第二个参数：" NewParam2)))

(event `API_ThreeParam`
  (params (NewParam :type String) (NewParam2 :type String) (NewParam3 :type String))
  (`KismetSystemLibrary.PrintString` (`KismetStringLibrary.Concat_StrStr` "第一个参数：" NewParam "   第二个参数：" NewParam2 "   第三个参数：   " NewParam3)))

(fn `API_Test_Func`
  (params (In5 :type String))
  (`KismetSystemLibrary.PrintString` (`KismetStringLibrary.Concat_StrStr` "In5：" In5)))

(fn `UserConstructionScript`)