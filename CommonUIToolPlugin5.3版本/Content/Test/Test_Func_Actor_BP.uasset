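; Test actor for calling functions by name and inspecting their parameters through reflection-style helper nodes.
; A custom event looks up API_Test_Func on the object in NewVar and invokes it with a JSON string argument.
; BeginPlay is empty, and disconnected chains hold experiments that call by name or print parameter names and types.
; A separate Test function prints its input and returns three fixed booleans.
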(event `self.ReceiveBeginPlay`)

(event `CustomEvent`
  (bind _newvar (`self.NewVar`))
  (`CommonUIToolLib.CallHaveParamsFunction` _newvar (`CommonUIToolLib.GetObjectFunction` _newvar "API_Test_Func") "{\"In5\":\"这是一个测试字符串\"}"))

(fn `Test`
  (params (NewParam :type String))
  (returns (NewParam1 :type Boolean) (NewParam2 :type Boolean) (NewParam3 :type Boolean))
  (`KismetSystemLibrary.PrintString` (`KismetStringLibrary.Concat_StrStr` "传入：" NewParam))
  (return false true false))

(fn `UserConstructionScript`)